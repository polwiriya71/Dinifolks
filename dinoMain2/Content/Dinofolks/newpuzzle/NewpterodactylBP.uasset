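; Pterodactyl quest NPC that starts collapsed and gets up once the player approaches after the meat's GetFood flag is set.
; Box overlap with the player checks the first Meat_Blueprint found, playing either a looping roar or a get-up-to-idle sequence, each with a one-time sound.
; Leaving the box replays the die animation unless it is up.
; Tick drives nameplate, quest marker and text visibility from the Inbox, GetUp and Q1complete flags.
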(event `Seeplayer`
  (`MovementComponent.StopMovementImmediately` (`self.CharacterMovement`))
  (bind _outactors (`GameplayStatics.GetAllActorsOfClass` "/Game/Dinofolks/texture/meat/meat_Blueprint.meat_Blueprint_C"))
  (if (`/Game/Dinofolks/texture/meat/meat_Blueprint.GetFood?` (`|GetArrayItem` _outactors))
    (`/Engine/EditorBlueprintResources/StandardMacros.DoOnce` false
      (:`Completed`
        (`SkeletalMeshComponent.PlayAnimation` (`self.Mesh`) "/Game/Toon_Dinosaurs/Pterodactyl/Animations/AnimationSequence_PterodactylGetUp.AnimationSequence_PterodactylGetUp" false)
        (`KismetSystemLibrary.Delay` 1.5)
        (`SkeletalMeshComponent.PlayAnimation` (`self.Mesh`) "/Game/Toon_Dinosaurs/Pterodactyl/Animations/AnimationSequence_PterodactylIdle.AnimationSequence_PterodactylIdle" true)
        (set `self.get up ?` true)
        (`SceneComponent.SetVisibility` (`self.T2`) true false)
        (`/Engine/EditorBlueprintResources/StandardMacros.DoOnce` false
          (:`Completed`
            (`GameplayStatics.PlaySound2D` "/Game/Dinofolks/UI/bird2.bird2" 1.0 1.0 0.0 null null)))))
    (else
      (`SkeletalMeshComponent.PlayAnimation` (`self.Mesh`) "/Game/Toon_Dinosaurs/Pterodactyl/Animations/AnimationSequence_PterodactylRoar.AnimationSequence_PterodactylRoar" true)
      (`/Engine/EditorBlueprintResources/StandardMacros.DoOnce` false
        (:`Completed`
          (`GameplayStatics.PlaySound2D` "/Game/Dinofolks/UI/bird1.bird1" 1.0 1.0 0.0 null null))))))

(event `self.ReceiveBeginPlay`
  (`SkeletalMeshComponent.PlayAnimation` (`self.Mesh`) "/Game/Toon_Dinosaurs/Pterodactyl/Animations/AnimationSequence_PterodactylDie.AnimationSequence_PterodactylDie" false))

(event `self.Box.OnComponentBeginOverlap`
  (params (OverlappedComponent :type "PrimitiveComponent Object Reference") (OtherActor :type "Actor Object Reference") (OtherComp :type "PrimitiveComponent Object Reference") (OtherBodyIndex :type Integer) (bFromSweep :type Boolean) (SweepResult :type "HitResult Structure (by ref)"))
  (cast `/Game/Dinofolks/gravity/Player` OtherActor)
  (`self.Seeplayer`)
  (set `self.inbox` true))

(event `self.ReceiveTick`
  (params (DeltaSeconds :type "Float (single-precision)"))
  (if (`self.inbox`)
    (`SceneComponent.SetVisibility` (`self.Nameplate`) true false)
    (`SceneComponent.SetVisibility` (`self.Q1`) true false)
    (`SceneComponent.SetVisibility` (`self.mark`) false false)
    (`SceneComponent.SetVisibility` (`self.T1`) true false)
    (if (`self.get up ?`)
      (`SceneComponent.SetVisibility` (`self.Q1`) false false)
      (`SceneComponent.SetVisibility` (`self.mark`) false false)
      (`SceneComponent.SetVisibility` (`self.T1`) false false)
      (set `self.q1complete` true)
      (`SceneComponent.SetVisibility` (`self.T2`) true false)
      (elif (`self.q1complete`)
        (`SceneComponent.SetVisibility` (`self.Q1`) false false)
        (`SceneComponent.SetVisibility` (`self.mark`) false false)
        (`SceneComponent.SetVisibility` (`self.T1`) false false)))
    (else
      (`SceneComponent.SetVisibility` (`self.Nameplate`) false false)
      (`SceneComponent.SetVisibility` (`self.Q1`) false false)
      (`SceneComponent.SetVisibility` (`self.T1`) false false)
      (`SceneComponent.SetVisibility` (`self.T2`) false false)
      (if (`self.get up ?`)
        (`SceneComponent.SetVisibility` (`self.Q1`) false false)
        (`SceneComponent.SetVisibility` (`self.mark`) false false)
        (`SceneComponent.SetVisibility` (`self.T1`) false false)
        (set `self.q1complete` true)
        (elif (`self.q1complete`)
          (`SceneComponent.SetVisibility` (`self.Q1`) false false)
          (`SceneComponent.SetVisibility` (`self.mark`) false false))))))

(event `self.Box.OnComponentEndOverlap`
  (params (OverlappedComponent :type "PrimitiveComponent Object Reference") (OtherActor :type "Actor Object Reference") (OtherComp :type "PrimitiveComponent Object Reference") (OtherBodyIndex :type Integer))
  (cast `/Game/Dinofolks/gravity/Player` OtherActor)
  (`self.Cantseeplayer`)
  (set `self.inbox` false))

(event `Cantseeplayer`
  (`MovementComponent.StopMovementImmediately` (`self.CharacterMovement`))
  (if (not (`self.get up ?`))
    (`SkeletalMeshComponent.PlayAnimation` (`self.Mesh`) "/Game/Toon_Dinosaurs/Pterodactyl/Animations/AnimationSequence_PterodactylDie.AnimationSequence_PterodactylDie" false)))

(fn `Display Nameplate`
  (`SceneComponent.SetVisibility` (`self.Nameplate`) true false))

(fn `Display Nameplate2`
  (`SceneComponent.SetVisibility` (`self.Q1`) true false))

(fn `UserConstructionScript`)